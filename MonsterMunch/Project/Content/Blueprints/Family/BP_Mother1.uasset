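; BP_Mother1 is the mother family member, an enemy that investigates checked points for the player.
; BeginPlay passes her spawn, timing, fail-chance and fake-out settings to Initialise, which also assigns the mum flipbooks, then matches the flipbook to her state.
; Investigation checks points for player occupancy and waits a random time.
; A second stage resets her state, notifies the door, updates the flipbook and clears the points' unsafe flags.
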(event EventBeginPlay
  (|CallParentFunction)
  (CallFunction|Initialise (Variables|Default|GetMySpawnTime) (Variables|Default|GetMyScoreSpawnThreshold) (Variables|Default|GetMyMinInvTime) (Variables|Default|GetMyMaxInvTime) (Variables|Default|GetMyMinS0ChangeDelay) (Variables|Default|GetMyMaxS0ChangeDelay) (Variables|Default|GetMyMinSChangeDelay%20%28Door%20Hold%29) (Variables|Default|GetMyMaxSChangeDelay%20%28Door%20Hold%29) (Variables|Default|GetMyFailChance) (Variables|Default|GetMyMinFakeOutTime) (Variables|Default|GetMyMaxFakeOutTime))
  (CallFunction|AdjustFlipbooktoState))

(fn ConstructionScript
  (|CallParentFunction))

(fn Initialise
  (params (Spawn%20Time%20%28Seconds%29 :type Float%20%28single-precision%29) (Score%20Spawn%20Threshold :type Integer) (Min%20Investigation%20Time :type Float%20%28single-precision%29) (Max%20Investigation%20Time :type Float%20%28single-precision%29) (Min%20State%200%20Change%20Delay :type Float%20%28single-precision%29) (Max%20State%200%20Change%20Delay :type Float%20%28single-precision%29) (Min%20State%20Change%20Delay :type Float%20%28single-precision%29) (Max%20State%20Change%20Delay :type Float%20%28single-precision%29) (Fail%20Chance%20%280.0%20-%201.0%29 :type Float%20%28single-precision%29) (Min%20Fake%20Out%20Time :type Float%20%28single-precision%29) (Max%20Fake%20Out%20Time :type Float%20%28single-precision%29))
  (Utilities|FlowControl|Sequence
    (:then_0
      (Variables|Default|SetSpawnTime Spawn%20Time%20%28Seconds%29))
    (:then_1
      (Variables|Default|SetScoreSpawnThreshold Score%20Spawn%20Threshold))
    (:then_2
      (Variables|Default|SetMinInvestigationTime Min%20Investigation%20Time))
    (:then_3
      (Variables|Default|SetMaxInvestigationTime Max%20Investigation%20Time))
    (:then_4
      (Variables|Default|SetMin%20State%200%20Change%20Delay Min%20State%200%20Change%20Delay))
    (:then_5
      (Variables|Default|SetMax%20State%200%20Change%20Delay Max%20State%200%20Change%20Delay))
    (:then_6
      (Variables|Default|SetMin%20State%20Change%20Delay Min%20State%20Change%20Delay))
    (:then_7
      (Variables|Default|SetMax%20State%20Change%20Delay Max%20State%20Change%20Delay))
    (:then_8
      (Variables|Default|SetMinFakeOutTime Min%20Fake%20Out%20Time))
    (:then_9
      (Variables|Default|SetMaxFakeOutTime Max%20Fake%20Out%20Time))
    (:then_10
      (Variables|Default|SetFail%20Chance Fail%20Chance%20%280.0%20-%201.0%29))
    (:then_11
      (Variables|Default|SetFlipbook%20Array (Variables|Default|GetMumFlipbooks)))))

(fn LerpAtoBActor0
  (params (Alpha :type Float%20%28single-precision%29) (A :type Vector) (B :type Vector))
  (Transformation|SetActorLocation (Math|Vector|Lerp(Vector) A B Alpha) false false))