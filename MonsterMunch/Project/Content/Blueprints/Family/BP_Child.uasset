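; BP_Child is the kid member of the game's family characters, configuring inherited spawn, investigation and state-change behaviour.
; On BeginPlay it runs the parent logic, then passes its own tuning variables to Initialise for spawn time, score threshold, timing ranges and fail chance.
; Initialise also assigns the kid flipbook array, after which AdjustFlipbookToState updates the sprite.
; Tick and construction only call the parent.
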(event EventBeginPlay
  (|CallParentFunction)
  (CallFunction|Initialise (Variables|Default|GetMySpawnTime) (Variables|Default|GetMyScoreSpawnThreshold) (Variables|Default|GetMyMinInvTime) (Variables|Default|GetMyMaxInvTime) (Variables|Default|GetMyMinSChangeDelay) (Variables|Default|GetMyMaxSChangeDelay) (Variables|Default|GetMyMaxS0ChangeDelay) (Variables|Default|GetMyFailChance))
  (CallFunction|AdjustFlipbooktoState))

(event EventTick
  (params (DeltaSeconds :type Float%20%28single-precision%29))
  (|CallParentFunction DeltaSeconds))

(fn ConstructionScript
  (|CallParentFunction))

(fn Initialise
  (params (Spawn%20Time%20%28Seconds%29 :type Float%20%28single-precision%29) (Score%20Spawn%20Threshold :type Integer) (Min%20Investigation%20time :type Float%20%28single-precision%29) (Max%20Investigation%20Time :type Float%20%28single-precision%29) (Min%20State%20Change%20Delay :type Float%20%28single-precision%29) (Max%20State%20Change%20Delay :type Float%20%28single-precision%29) (Max%20State%200%20Change%20Delay :type Float%20%28single-precision%29) (Fail%20Chance%20%280.0%20-%201.0%29 :type Float%20%28single-precision%29))
  (Utilities|FlowControl|Sequence
    (:then_0
      (Variables|Default|SetSpawnTime Spawn%20Time%20%28Seconds%29))
    (:then_1
      (Variables|Default|SetScoreSpawnThreshold Score%20Spawn%20Threshold))
    (:then_2
      (Variables|Default|SetMinInvestigationTime Min%20Investigation%20time))
    (:then_3
      (Variables|Default|SetMaxInvestigationTime Max%20Investigation%20Time))
    (:then_4
      (Variables|Default|SetMin%20State%20Change%20Delay Min%20State%20Change%20Delay))
    (:then_5
      (Variables|Default|SetMax%20State%20Change%20Delay Max%20State%20Change%20Delay))
    (:then_6
      (Variables|Default|SetMax%20State%200%20Change%20Delay Max%20State%200%20Change%20Delay))
    (:then_7
      (Variables|Default|SetFail%20Chance Fail%20Chance%20%280.0%20-%201.0%29))
    (:then_8
      (Variables|Default|SetFlipbook%20Array (Variables|Default|GetKid%20Flipbook)))))