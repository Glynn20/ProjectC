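; Player camera Blueprint that runs the core game: point-to-point movement, fridge eating, scoring and game over.
; WASD and Space teleport the player between placed points; hanging at the Space point drains grip, and running out triggers a fatal fall.
; Holding E scores through a delayed self-calling loop, while a multiplier loop speeds scoring up during eating.
; It also drives the score UI, hide fades and high-score saving.
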(event Custom|Begin%20Multiplier
  (if (Variables|Default|GetIsEating) :!label _label
    (Variables|Default|SetFunctionRate 1.2)
    (else
      (Variables|Default|SetFunctionRate 0.6)))
  (Utilities|FlowControl|Delay (Variables|Default|GetFunctionRate))
  (Utilities|AdjustMultiplier (Variables|Default|GetIsEating)
    (:NewParam
      (goto _label))))

(event Custom|Grip%20+
  ;[1 1 1] Grip System
  (if (not (Variables|Default|GetIsGripping))
    (if (not (>= (Variables|Default|GetGrip) (Variables|Default|GetMaxGrip)))
      (bind _output_get (Variables|Default|SetGrip (+ (Variables|Default|GetGrip) 2)))
      (CallFunction|AdjustGripMeterPercent (Math|Conversions|ToFloat(Integer) _output_get))
      (Utilities|FlowControl|Delay 0.2)
      (CallFunction|Grip+))))

(event Custom|Game%20Over
  ;[1 1 1] New Game over to be implemented
  (Input|DisableInput 0)
  (CallFunction|SetHighScore)
  (Default|GameOverUI (Variables|Default|GetUIScore))
  (CameraFades|StartCameraFade :self (Game|GetPlayerCameraManager 0) :ToAlpha 1.0 :Duration 0.8 :bShouldFadeAudio true :bHoldWhenFinished true)
  (Utilities|FlowControl|Delay 4.0)
  (Game|OpenLevel(byName) "MainMenu"))

(event Custom|Grip%20-
  ;[1 1 1] Grip System
  (if (Variables|Default|GetIsGripping)
    (if (<= (Variables|Default|GetGrip) 0)
      (Variables|Default|SetIsGripping false)
      (bind _output_get (Variables|Default|SetPlayerLocation (Transformation|GetActorLocation (Variables|Default|GetPlayerRef))))
      (Audio|PlaySoundatLocation "/Game/Sounds/Player/SC_PlayerFall.SC_PlayerFall" _output_get "0, 0, 0" 1.0 1.0 0.0 0 0 0)
      (bind _newtrack_0 (Timeline|Timeline_0 PlayFromStart)
        (:Update
          (CallFunction|LerpAtoBActor _newtrack_0 _output_get (Variables|Default|GetSLocation) (Variables|Default|GetPlayerRef)))
        (:Finished
          (Utilities|PlayerFallsandDies)))
      (else
        (bind _output_get_2 (Variables|Default|SetGrip (- (Variables|Default|GetGrip) (Variables|Default|GetGripDecreaseRate))))
        (CallFunction|AdjustGripMeterPercent (Math|Conversions|ToFloat(Integer) _output_get_2))
        (Utilities|FlowControl|Delay 0.2)
        (CallFunction|Grip-)))))

(event Custom|Eat
  ;[1 1 1] Eat
  (if (Variables|Default|GetIsEating)
    (bind _asfridge (Utilities|Casting|CastToFridge (Variables|Default|GetFridgeRef)))
    (if (Variables|/Game/Blueprints/Gamemode/Fridge.Fridge_C|GetCanEat _asfridge)
      (bind _output_get (Variables|Default|SetScore (+ 1 (Variables|Default|GetScore))))
      (CallFunction|EatSound (Variables|Default|GetPlayerRef))
      (Default|UpdateScore (Variables|Default|GetUIScore) _output_get)
      (Utilities|FlowControl|Delay (Variables|Default|GetScoring%20Rate))
      (CallFunction|Eat))))

(event Custom|Enable%20Hide%20Effect
  (CameraFades|StartCameraFade (Game|GetPlayerCameraManager 0) 0.0 0.55 0.2 "(R=0.000000,G=0.000000,B=0.000000,A=1.000000)" true true)
  (Audio|PlaySoundatLocation "/Game/Sounds/Player/SC_PlayerHide.SC_PlayerHide" "0, 0, 0" "0, 0, 0" 1.0 1.0 0.0 0 0 0))

(event Custom|Remove%20Hide%20Effect
  (if (Variables|Default|GetIsHiding)
    (CameraFades|StartCameraFade (Game|GetPlayerCameraManager 0) 0.6 0.0 0.2 "(R=0.000000,G=0.000000,B=0.000000,A=1.000000)" true true)
    (Variables|Default|SetIsHiding false)))

(event EventBeginPlay
  (CallFunction|InitVariables)
  (bind _returnvalue (UserInterface|CreateWidget "/Game/Blueprints/UI/UI_Score.UI_Score_C"))
  (bind _output_get (Variables|Default|SetUIScore _returnvalue))
  (UserInterface|Viewport|AddtoViewport _output_get 0)
  (CallFunction|BeginMultiplier))

(event Input|KeyboardEvents|W
  (params (Key :type Key%20Structure :default "None"))
  ;[1 1 1] PlayerMovement
  (:Pressed
    (CallFunction|MovetoPoint (Variables|Default|GetWLocation))))

(event Input|KeyboardEvents|A
  (params (Key :type Key%20Structure :default "None"))
  ;[1 1 1] PlayerMovement
  (:Pressed
    (CallFunction|MovetoPoint (Variables|Default|GetALocation))))

(event Input|KeyboardEvents|S
  (params (Key :type Key%20Structure :default "None"))
  ;[1 1 1] PlayerMovement
  (:Pressed
    (CallFunction|MovetoPoint (Variables|Default|GetSLocation))))

(event Input|KeyboardEvents|D
  (params (Key :type Key%20Structure :default "None"))
  ;[1 1 1] PlayerMovement
  (:Pressed
    (CallFunction|MovetoPoint (Variables|Default|GetDLocation))))

(event Input|KeyboardEvents|E
  (params (Key :type Key%20Structure :default "None"))
  ;[1 1 1] Eat
  (:Pressed
    (Variables|Default|SetIsEating true)
    (CallFunction|Eat))
  (:Released
    (Variables|Default|SetIsEating false)))

(event Input|KeyboardEvents|SpaceBar
  (params (Key :type Key%20Structure :default "None"))
  ;[1 1 1] Grip System
  (:Pressed
    (CallFunction|MovetoPoint (Variables|Default|GetSpacebarLocation))
    (Audio|PlaySoundatLocation "/Game/Sounds/Player/SC_PlayerRopeHang.SC_PlayerRopeHang" "0, 0, 0" "0, 0, 0" 1.0 1.0 0.0 0 0 0))
  (:Released
    (CallFunction|ReleaseGrip)
    (bind _result (CallFunction|CheckifatSpacePoint))
    (if _result
      (CallFunction|MovetoPoint (Variables|Default|GetSLocation)))))

(fn ConstructionScript)

(fn InitVariables
  (Variables|Default|SetWLocation (Transformation|GetActorLocation (Variables|Default|GetWPoint)))
  (Variables|Default|SetALocation (Transformation|GetActorLocation (Variables|Default|GetAPoint)))
  (Variables|Default|SetSLocation (Transformation|GetActorLocation (Variables|Default|GetSPoint)))
  (Variables|Default|SetDLocation (Transformation|GetActorLocation (Variables|Default|GetDPoint)))
  (Variables|Default|SetSpacebarLocation (Transformation|GetActorLocation (Variables|Default|GetSpacebarPoint)))
  (Variables|Default|SetPlayerLocation (Transformation|GetActorLocation (Variables|Default|GetPlayerRef))))

(fn MovetoPoint
  (params (PointLocation :type Vector))
  (Transformation|Teleport (Variables|Default|GetPlayerRef) PointLocation "0, 0, 0")
  (Audio|PlaySoundatLocation "/Game/Sounds/Player/SC_PlayerMove.SC_PlayerMove" "0, 0, 0" "0, 0, 0" 1.0 1.0 0.0 0 0 0)
  (bind _result (CallFunction|CheckifatSpacePoint))
  (if _result
    (CallFunction|BeginGrip)
    (else
      (CallFunction|ReleaseGrip))))

(fn EatSound
  (params (self2 :type Actor%20Object%20Reference))
  (Audio|PlaySoundatLocation "/Game/Sounds/Player/PlayerMunch.PlayerMunch" (Transformation|GetActorLocation self2) "0, 0, 0" 0.8 0.95 0.0 0 0 0))

(fn LerpAtoBActor
  (params (Alpha :type Float%20%28single-precision%29) (A :type Vector) (B :type Vector) (Actor :type Actor%20Object%20Reference))
  (Transformation|SetActorLocation Actor (Math|Vector|Lerp(Vector) A B Alpha) false false))

(fn AdjustGripMeterPercent
  (params (A :type Float%20%28single-precision%29))
  (Progress|SetPercent (Variables|/Game/Blueprints/UI/UI_Score.UI_Score_C|GetProgressBar_131 (Variables|Default|GetUIScore)) (Math|Float|SafeDivide A 1e+02)))

(fn ReleaseGrip
  (Variables|Default|SetIsGripping false)
  (CallFunction|Grip+))

(fn BeginGrip
  (Variables|Default|SetIsGripping true)
  (CallFunction|Grip-))

(fn CheckifatSpacePoint
  (bind _aspoints (Utilities|Casting|CastToPoints (Variables|Default|GetSpacebarPoint)))
  (return (Variables|/Game/Blueprints/MoveablePoints/Player/Points.Points_C|GetPlayerOccupied _aspoints)))

(fn SetHighScore
  (bind _returnvalue (SaveGame|DoesSaveGameExist "HS"))
  (if _returnvalue
    (bind _returnvalue_2 (SaveGame|LoadGamefromSlot "HS"))
    (bind _assg_high_score (Utilities|Casting|CastToSG_HighScore _returnvalue_2))
    (if (> (Variables|Default|GetScore) (Variables|/Game/Blueprints/Player/SG_HighScore.SG_HighScore_C|GetHigh%20Score _assg_high_score))
      (bind _returnvalue_3 (SaveGame|CreateSaveGameObject "/Game/Blueprints/Player/SG_HighScore.SG_HighScore_C" :!label _label))
      (Variables|/Game/Blueprints/Player/SG_HighScore.SG_HighScore_C|SetHigh%20Score _returnvalue_3 (Variables|Default|GetScore))
      (SaveGame|SaveGametoSlot _returnvalue_3 "HS"))
    (else
      (goto _label))))