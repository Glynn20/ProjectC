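; BP_Door is a door actor that opens and closes in response to its owner, either a mother or a child character.
; When the mother changes state, it snaps to one of three preset rotations, plays that state's sound and prints a debug string.
; When the child begins or stops investigating, it snaps to its Open or Closed rotation.
; Each event casts OwnerRef, so it only acts for the matching owner type.
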(event Custom|Mum%20has%20Changed%20State
  (bind _asbp_mother_1 (Utilities|Casting|CastToBP_Mother1 (Variables|Default|GetOwnerRef)))
  (CallFunction|AdjustStateBasedonMum (Variables|/Game/Blueprints/Family/BP_Family1.BP_Family1_C|GetState _asbp_mother_1)))

(event Custom|Child%20Stops%20Investigation
  (Utilities|Casting|CastToBP_Child (Variables|Default|GetOwnerRef))
  (Transformation|SetActorRotation (Variables|Default|GetClosed)))

(event Custom|Child%20Begins%20Investigation
  (Utilities|Casting|CastToBP_Child (Variables|Default|GetOwnerRef))
  (Transformation|SetActorRotation (Variables|Default|GetOpen)))

(fn ConstructionScript)

(fn AdjustStateBasedonMum
  (params (State :type Integer))
  (Transformation|SetActorRotation (Utilities|Select :Index State :Option%200 "0, 0, 0" :Option%201 "0,30.000000, 0" :Option%202 "0,90.000000, 0"))
  (Audio|PlaySoundatLocation (Utilities|Array|Get(acopy) (Variables|Default|GetMySounds) State) (Transformation|GetActorLocation) "0, 0, 0" 1.3 1.0 0.0 0 0 0)
  (Development|PrintString "Hello"))