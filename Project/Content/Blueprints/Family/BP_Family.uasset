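; BP_Family is a Blueprint that drives an integer State on a randomized timer loop started at BeginPlay.
; Each pass waits briefly, adds a longer random delay unless State is 1 or 2, then calls ChangeState.
; ChangeState randomly either resets State to zero or increments it with no upper limit, printing the result.
; TryMove is an empty stub, with a Difficulty-based random roll left unconnected.
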(event Custom|Change%20State
  (if (< (Math|Random|RandomIntegerinRange 0 10) 3)
    (Variables|Default|SetState 0) ; Reset to 0
    (Development|PrintString "Reset to 0")
    (else
      (Variables|Default|SetState (+ (Variables|Default|GetState) 1))
      (Development|PrintString "increment state")
      (if true
        _))))

(event EventBeginPlay
  (bind _state (Variables|Default|GetState))
  (Utilities|FlowControl|Delay (Math|Random|RandomFloatinRange 0.8 0.9) :!label _label)
  (if (and (> _state 0) (< _state 3))
    _
    (else
      (Utilities|FlowControl|Delay (Math|Random|RandomFloatinRange 5.0 1e+01))))
  (CallFunction|ChangeState)
  (goto _label))

(fn ConstructionScript)

(fn TryMove)

(fn Resetto0
  (Variables|Default|SetState 0) ; Reset to 0
)