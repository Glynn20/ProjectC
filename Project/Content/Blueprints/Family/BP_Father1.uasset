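; BP_Father1 is the father variant of a family character that spawns and investigates, built on a parent class that provides the state behaviour.
; On BeginPlay it passes its tuning for spawning, investigation time, state-change delays and fail chance, plus the dad flipbook set, into inherited variables, then refreshes the flipbook.
; A looping one-minute timer plays ambient radio audio at the actor's location.
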(event EventBeginPlay
  (|CallParentFunction)
  (CallFunction|Initialise (Variables|Default|GetMySpawnTime) (Variables|Default|GetMyScoreSpawnThreshold) (Variables|Default|GetMyMinInvTime) (Variables|Default|GetMyMaxInvTime) (Variables|Default|GetMyMaxSChangeDelay) (Variables|Default|GetMyMaxS0ChangeDelay) (Variables|Default|GetMyFailChance) (Variables|Default|GetMyMinSChangeDelay))
  (CallFunction|AdjustFlipbooktoState)
  (Utilities|Time|SetTimerbyFunctionName 0 "Play Radio" 6e+01 true))

(event EventTick
  (params (DeltaSeconds :type Float%20%28single-precision%29))
  (|CallParentFunction DeltaSeconds))

(fn ConstructionScript
  (|CallParentFunction))

(fn Initialise
  (params (SpawnTime%20%28Seconds%29 :type Float%20%28single-precision%29) (ScoreSpawnThreshold :type Integer) (MinInvestigationTime :type Float%20%28single-precision%29) (MaxInvestigationTime :type Float%20%28single-precision%29) (MaxStateChangeDelay :type Float%20%28single-precision%29) (MaxState%200%20ChangeDelay :type Float%20%28single-precision%29) (FailChance%20%280.0%20-%201.0%29 :type Float%20%28single-precision%29) (Min%20State%20Change%20Delay :type Float%20%28single-precision%29))
  (Utilities|FlowControl|Sequence
    (:then_0
      (Variables|Default|SetSpawnTime SpawnTime%20%28Seconds%29))
    (:then_1
      (Variables|Default|SetScoreSpawnThreshold ScoreSpawnThreshold))
    (:then_2
      (Variables|Default|SetMinInvestigationTime MinInvestigationTime))
    (:then_3
      (Variables|Default|SetMaxInvestigationTime MaxInvestigationTime))
    (:then_4
      (Variables|Default|SetMax%20State%20Change%20Delay MaxStateChangeDelay))
    (:then_5
      (Variables|Default|SetMax%20State%200%20Change%20Delay MaxState%200%20ChangeDelay))
    (:then_6
      (Variables|Default|SetFail%20Chance FailChance%20%280.0%20-%201.0%29))
    (:then_7
      (Variables|Default|SetFlipbook%20Array (Variables|Default|GetDad%20Flipbook)))
    (:then_8
      (Variables|Default|SetMin%20State%20Change%20Delay Min%20State%20Change%20Delay))))

(fn PlayRadio
  (Audio|PlaySoundatLocation "/Game/Sounds/Ambient_Radio.Ambient_Radio" (Transformation|GetActorLocation) "0, 0, 0" 1.0 1.0 0.0 0 0 0))