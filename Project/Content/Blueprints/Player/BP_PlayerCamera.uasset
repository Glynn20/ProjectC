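; Player camera Blueprint that runs the core loop: input, hiding fade, fridge-eating score, grip and game over.
; WASD and Spacebar teleport the referenced player actor between placed points; holding Spacebar drains grip, and running out triggers a timeline fall, death and quit.
; Holding E scores through a delayed recursive loop while the fridge allows it.
; A separate loop ramps eating speed and multiplier up while eating, down otherwise, updating the score widget.
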(event Custom|Begin%20Multiplier
  (if (Variables|Default|GetIsEating) :!label _label
    (Variables|Default|SetFunctionRate 1.2)
    (else
      (Variables|Default|SetFunctionRate 0.6)))
  (Utilities|FlowControl|Delay (Variables|Default|GetFunctionRate))
  (Utilities|AdjustMultiplier (Variables|Default|GetIsEating)
    (:NewParam
      (goto _label))))

(event Custom|Grip%20+
  ;[1 1 1] Grip System
  (if (not (Variables|Default|GetIsGripping))
    (if (not (>= (Variables|Default|GetGrip) (Variables|Default|GetMaxGrip)))
      (bind _output_get (Variables|Default|SetGrip (+ (Variables|Default|GetGrip) 2)))
      (Development|PrintString (Utilities|String|ToString(Integer) _output_get))
      (Utilities|FlowControl|Delay 0.2)
      (CallFunction|Grip+))))

(event Custom|Game%20Over
  ;[1 1 1] New Game over to be implemented
  (Input|DisableInput 0)
  (CameraFades|StartCameraFade :self (Game|GetPlayerCameraManager 0) :ToAlpha 1.0 :Duration 0.8 :bShouldFadeAudio true :bHoldWhenFinished true)
  (Utilities|FlowControl|Delay 1.0)
  (Default|GameOverUI (Variables|Default|GetUIScore))
  (Utilities|FlowControl|Delay 4.0)
  (Game|QuitGame 0 "Quit" false))

(event Custom|Grip%20-
  ;[1 1 1] Grip System
  (if (Variables|Default|GetIsGripping)
    (if (<= (Variables|Default|GetGrip) 0)
      (Variables|Default|SetIsGripping false)
      (bind _output_get (Variables|Default|SetPlayerLocation (Transformation|GetActorLocation (Variables|Default|GetPlayerRef))))
      (Audio|PlaySoundatLocation "/Game/Sounds/Player/SC_PlayerFall.SC_PlayerFall" _output_get "0, 0, 0" 1.0 1.0 0.0 0 0 0)
      (bind _newtrack_0 (Timeline|Timeline_0 PlayFromStart)
        (:Update
          (CallFunction|LerpAtoBActor _newtrack_0 _output_get (Variables|Default|GetSLocation) (Variables|Default|GetPlayerRef)))
        (:Finished
          (Utilities|PlayerFallsandDies)))
      (else
        (bind _output_get_2 (Variables|Default|SetGrip (- (Variables|Default|GetGrip) (Variables|Default|GetGripDecreaseRate))))
        (Development|PrintString (Utilities|String|ToString(Integer) _output_get_2))
        (Utilities|FlowControl|Delay 0.2)
        (CallFunction|Grip-)))))

(event Custom|Eat
  ;[1 1 1] Eat
  (if (Variables|Default|GetIsEating)
    (bind _asfridge (Utilities|Casting|CastToFridge (Variables|Default|GetFridgeRef)))
    (if (Variables|/Game/Blueprints/Gamemode/Fridge.Fridge_C|GetCanEat _asfridge)
      (bind _output_get (Variables|Default|SetScore (+ 1 (Variables|Default|GetScore))))
      (CallFunction|EatSound (Variables|Default|GetPlayerRef))
      (Default|UpdateScore (Variables|Default|GetUIScore) _output_get)
      (Utilities|FlowControl|Delay (Variables|Default|GetScoring%20Rate))
      (CallFunction|Eat))))

(event Custom|Enable%20Hide%20Effect
  (CameraFades|StartCameraFade (Game|GetPlayerCameraManager 0) 0.0 0.55 0.2 "(R=0.000000,G=0.000000,B=0.000000,A=1.000000)" true true)
  (Audio|PlaySoundatLocation "/Game/Sounds/Player/SC_PlayerHide.SC_PlayerHide" "0, 0, 0" "0, 0, 0" 1.0 1.0 0.0 0 0 0))

(event Custom|Remove%20Hide%20Effect
  (if (Variables|Default|GetIsHiding)
    (CameraFades|StartCameraFade (Game|GetPlayerCameraManager 0) 0.6 0.0 0.2 "(R=0.000000,G=0.000000,B=0.000000,A=1.000000)" true true)
    (Variables|Default|SetIsHiding false)))

(event EventBeginPlay
  (CallFunction|InitVariables)
  (bind _returnvalue (UserInterface|CreateWidget "/Game/Blueprints/UI/UI_Score.UI_Score_C"))
  (bind _output_get (Variables|Default|SetUIScore _returnvalue))
  (UserInterface|Viewport|AddtoViewport _output_get 0)
  (CallFunction|BeginMultiplier))

(event Input|KeyboardEvents|W
  (params (Key :type Key%20Structure :default "None"))
  ;[1 1 1] PlayerMovement
  (:Pressed
    (CallFunction|MovetoPoint (Variables|Default|GetWLocation))))

(event Input|KeyboardEvents|A
  (params (Key :type Key%20Structure :default "None"))
  ;[1 1 1] PlayerMovement
  (:Pressed
    (CallFunction|MovetoPoint (Variables|Default|GetALocation))))

(event Input|KeyboardEvents|S
  (params (Key :type Key%20Structure :default "None"))
  ;[1 1 1] PlayerMovement
  (:Pressed
    (CallFunction|MovetoPoint (Variables|Default|GetSLocation))))

(event Input|KeyboardEvents|D
  (params (Key :type Key%20Structure :default "None"))
  ;[1 1 1] PlayerMovement
  (:Pressed
    (CallFunction|MovetoPoint (Variables|Default|GetDLocation))))

(event Input|KeyboardEvents|E
  (params (Key :type Key%20Structure :default "None"))
  ;[1 1 1] Eat
  (:Pressed
    (Variables|Default|SetIsEating true)
    (CallFunction|Eat))
  (:Released
    (Variables|Default|SetIsEating false)))

(event Input|KeyboardEvents|SpaceBar
  (params (Key :type Key%20Structure :default "None"))
  ;[1 1 1] Grip System
  (:Pressed
    (CallFunction|MovetoPoint (Variables|Default|GetSpacebarLocation))
    (Audio|PlaySoundatLocation "/Game/Sounds/Player/SC_PlayerRopeHang.SC_PlayerRopeHang" "0, 0, 0" "0, 0, 0" 1.0 1.0 0.0 0 0 0)
    (Variables|Default|SetIsGripping true)
    (CallFunction|Grip-))
  (:Released
    (Variables|Default|SetIsGripping false)
    (CallFunction|Grip+)
    (CallFunction|MovetoPoint (Variables|Default|GetSLocation))))

(fn ConstructionScript)

(fn InitVariables
  (Variables|Default|SetWLocation (Transformation|GetActorLocation (Variables|Default|GetWPoint)))
  (Variables|Default|SetALocation (Transformation|GetActorLocation (Variables|Default|GetAPoint)))
  (Variables|Default|SetSLocation (Transformation|GetActorLocation (Variables|Default|GetSPoint)))
  (Variables|Default|SetDLocation (Transformation|GetActorLocation (Variables|Default|GetDPoint)))
  (Variables|Default|SetSpacebarLocation (Transformation|GetActorLocation (Variables|Default|GetSpacebarPoint)))
  (Variables|Default|SetPlayerLocation (Transformation|GetActorLocation (Variables|Default|GetPlayerRef))))

(fn MovetoPoint
  (params (PointLocation :type Vector))
  (Transformation|Teleport (Variables|Default|GetPlayerRef) PointLocation "0, 0, 0")
  (Audio|PlaySoundatLocation 0 "0, 0, 0" "0, 0, 0" 1.0 1.0 0.0 0 0 0))

(fn EatSound
  (params (self2 :type Actor%20Object%20Reference))
  (Audio|PlaySoundatLocation "/Game/Sounds/Player/PlayerMunch.PlayerMunch" (Transformation|GetActorLocation self2) "0, 0, 0" 0.8 0.95 0.0 0 0 0))

(fn LerpAtoBActor
  (params (Alpha :type Float%20%28single-precision%29) (A :type Vector) (B :type Vector) (Actor :type Actor%20Object%20Reference))
  (Transformation|SetActorLocation Actor (Math|Vector|Lerp(Vector) A B Alpha) false false))