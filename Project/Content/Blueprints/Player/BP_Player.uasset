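; Player Blueprint that reacts to fridges and hiding spots and handles losing the game.
; Overlap begin and end call SetFridge, which toggles CanEat on any overlapped Fridge.
; Overlapping a Points actor swaps the Monster sprite to hide or idle based on IsHidingSpot; ending overlap leaves the sprite unchanged.
; GameOver prints a loss message, waits briefly, then quits the game.
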(event Custom|Game%20Over
  (Development|PrintString "You Lost")
  (Utilities|FlowControl|Delay 5.0)
  (Game|QuitGame 0 "Quit" false))

(event Collision|EventActorEndOverlap
  (params (OtherActor :type Actor%20Object%20Reference))
  (CallFunction|SetFridge OtherActor false))

(event Collision|EventActorBeginOverlap
  (params (OtherActor :type Actor%20Object%20Reference))
  (bind _monster (Variables|Default|GetMonster))
  (CallFunction|SetFridge OtherActor true)
  (bind _aspoints (Utilities|Casting|CastToPoints OtherActor)) ; Fires if Not Fridge
  (if (Variables|/Game/Blueprints/MoveablePoints/Player/Points.Points_C|GetIsHidingSpot _aspoints)
    (Rendering|Components|Sprite|SetSprite _monster "/Game/Sprites/Player/Monster_Hide_Sprite.Monster_Hide_Sprite")
    (else
      (Rendering|Components|Sprite|SetSprite _monster "/Game/Sprites/Player/Monster_Idle_Sprite.Monster_Idle_Sprite"))))

(fn ConstructionScript)

(fn SetFridge
  (params (Object :type Object%20Object%20Reference) (State :type Boolean))
  (bind _asfridge (Utilities|Casting|CastToFridge Object)
    (:then
      (Variables|/Game/Blueprints/Gamemode/Fridge.Fridge_C|SetCanEat _asfridge State))
    (:CastFailed
      (return))))